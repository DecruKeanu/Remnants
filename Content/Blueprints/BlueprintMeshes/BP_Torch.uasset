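; BP_Torch is a torch Blueprint that returns its physics cylinder to its starting spot after it falls too far.
; BeginPlay stores the cylinder's world location, and Tick checks whether it has dropped more than MaxZDifference below that height.
; When it has, a two-second Delay runs before ResetPosition zeroes linear velocity and teleports the cylinder back, leaving rotation untouched.
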(event `self.ReceiveBeginPlay`
  ;[1 1 1] Saves startposition at the start of the game
  (set `self.StartPos` (`SceneComponent.K2_GetComponentLocation` (`self.Cylinder`))))

(event `ResetPosition`
  ;[1 1 1] resets position to startPos when called
  (`PrimitiveComponent.SetPhysicsLinearVelocity` (`self.Cylinder`) (0.0 0.0 0.0) false "None")
  (`SceneComponent.K2_SetWorldLocation` (`self.Cylinder`) (`self.StartPos`) false true))

(event `self.ReceiveTick`
  (params (DeltaSeconds :type "Float (single-precision)"))
  (bind (_startpos_x _startpos_y _startpos_z) (`KismetMathLibrary.BreakVector` (`self.StartPos`)))
  (bind (_returnvalue_x _returnvalue_y _returnvalue_z) (`KismetMathLibrary.BreakVector` (`SceneComponent.K2_GetComponentLocation` (`self.Cylinder`))))
  ;[1 1 1] Check if position needs to be reset
  (if (> (- _startpos_z (`self.MaxZDifference`)) _returnvalue_z)
    (`KismetSystemLibrary.Delay` 2.0)
    (`self.ResetPosition`)))

(fn `UserConstructionScript`)