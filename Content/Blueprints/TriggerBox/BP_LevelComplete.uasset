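; BP_LevelComplete is a trigger that ends the level when an actor begins overlapping it.
; On overlap it disables player input, fades the camera out and holds the fade, then after a matching delay shows the W_CompleteLevel widget, re-enables input and sets LevelCompleted.
; The overlap does not filter which actor entered, and the StartInteract and EndInteract functions are empty.
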(event `self.ReceiveActorBeginOverlap`
  (params (OtherActor :type "Actor Object Reference"))
  (bind _returnvalue (`GameplayStatics.GetPlayerController` 0))
  (bind _returnvalue_2 (`GameplayStatics.GetPlayerController` 0))
  ;[1 1 1] BeginOverlap
  (`self.DisableInput` _returnvalue _returnvalue)
  (`PlayerCameraManager.StartCameraFade` :`self` (`GameplayStatics.GetPlayerCameraManager` 0) :`ToAlpha` 1.0 :`Duration` 2.0 :`bHoldWhenFinished` true)
  (`KismetSystemLibrary.Delay` 2.0)
  (bind _returnvalue_3 (`|CreateWidget` "/Game/W_CompleteLevel.W_CompleteLevel_C"))
  (`UserWidget.AddToViewport` _returnvalue_3 0)
  (`self.EnableInput` _returnvalue_2 _returnvalue_2)
  (set `self.LevelCompleted` true))

(fn `EndInteract`
  (params (InputObject :type "/Game/Blueprints/TriggerBox/BP_TriggerParent Object Reference"))
  (returns (Player :type "/Game/Blueprints/BP_PlayerCharacter Object Reference"))
  (return null))

(fn `StartInteract`
  (params (InputObject :type "/Game/Blueprints/TriggerBox/BP_TriggerParent Object Reference"))
  (returns (Player :type "/Game/Blueprints/BP_PlayerCharacter Object Reference"))
  (return null))

(fn `UserConstructionScript`)