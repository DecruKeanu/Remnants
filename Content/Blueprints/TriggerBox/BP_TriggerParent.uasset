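; Base interactable trigger, apparently meant as a parent for other triggers, that shows or hides a text prompt around overlaps.
; Begin and end overlap send start and end interact messages with itself to player pawn 0 and toggle the TextRender, without filtering the overlapping actor.
; The Interactwith event and Interaction function both call CheckInteraction.
; Its own StartInteract and EndInteract functions are empty.
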(event `self.ReceiveActorBeginOverlap`
  (params (OtherActor :type "Actor Object Reference"))
  ;[1 1 1] BeginOverlap
  (message `/Game/Blueprints/BPI_Interaction.StartInteract` (`GameplayStatics.GetPlayerPawn` 0) self)
  (`SceneComponent.ToggleVisibility` (`self.TextRender`) false))

(event `self.ReceiveActorEndOverlap`
  (params (OtherActor :type "Actor Object Reference"))
  ;[1 1 1] EndOverlap
  (message `/Game/Blueprints/BPI_Interaction.EndInteract` (`GameplayStatics.GetPlayerPawn` 0) self)
  (`SceneComponent.ToggleVisibility` (`self.TextRender`) false))

(event `/Game/Blueprints/BPI_Interaction.InteractWith`
  ;[1 1 1] Interaction
  (`self.CheckInteraction`))

(fn `EndInteract`
  (params (InputObject :type "/Game/Blueprints/TriggerBox/BP_TriggerParent Object Reference"))
  (returns (Player :type "/Game/Blueprints/BP_PlayerCharacter Object Reference"))
  (return null))

(fn `Interaction`
  (`self.CheckInteraction`))

(fn `StartInteract`
  (params (InputObject :type "/Game/Blueprints/TriggerBox/BP_TriggerParent Object Reference"))
  (returns (Player :type "/Game/Blueprints/BP_PlayerCharacter Object Reference"))
  (return null))

(fn `UserConstructionScript`)