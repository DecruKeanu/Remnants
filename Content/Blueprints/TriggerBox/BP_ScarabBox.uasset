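; BP_ScarabBox is a trigger volume that disables the player's throwing and flashlight while inside and respawns them after a fall.
; Begin overlap records the player's location as the respawn point, and end overlap re-enables both abilities.
; While overlapping, Tick watches for the player dropping over 200 units below that point, then fades out, teleports them back and fades in.
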(event `self.ReceiveBeginPlay`
  (bind _asbp_player_character (cast `/Game/Blueprints/BP_PlayerCharacter` (`GameplayStatics.GetPlayerPawn` 0)))
  (set `self.PlayerCharacter` _asbp_player_character))

(event `self.ReceiveActorBeginOverlap`
  (params (OtherActor :type "Actor Object Reference"))
  (bind _playercharacter (`self.PlayerCharacter`))
  ;[1 1 1] Disables flashlight and throwing
  (if (== OtherActor _playercharacter)
    (set `self.RespawnLocation` (`self.K2_GetActorLocation` _playercharacter))
    (`/Game/Blueprints/BP_PlayerCharacter.DisableThrow` _playercharacter)
    (`/Game/Blueprints/BP_PlayerCharacter.DisableFlashlight` _playercharacter)
    (set `self.IsOverlapping` true)))

(event `self.ReceiveActorEndOverlap`
  (params (OtherActor :type "Actor Object Reference"))
  ;[1 1 1] Enables flashlight and throwing
  (bind _asbp_player_character (cast `/Game/Blueprints/BP_PlayerCharacter` OtherActor))
  (`/Game/Blueprints/BP_PlayerCharacter.Enablethrow` _asbp_player_character)
  (`/Game/Blueprints/BP_PlayerCharacter.EnableFlashlight` _asbp_player_character)
  (set `self.IsOverlapping` false))

(event `self.ReceiveTick`
  (params (DeltaSeconds :type "Float (single-precision)"))
  (bind (_respawnlocation_x _respawnlocation_y _respawnlocation_z) (`KismetMathLibrary.BreakVector` (`self.RespawnLocation`)))
  (bind (_returnvalue_x _returnvalue_y _returnvalue_z) (`KismetMathLibrary.BreakVector` (`self.K2_GetActorLocation` (`self.PlayerCharacter`))))
  ;[1 1 1] Handles player respawn
  (if (`self.IsOverlapping`)
    (if (> (- _respawnlocation_z 200.0) _returnvalue_z)
      (`PlayerCameraManager.StartCameraFade` :`self` (`GameplayStatics.GetPlayerCameraManager` 0) :`ToAlpha` 1.0 :`Duration` 1.5 :`bHoldWhenFinished` true)
      (`KismetSystemLibrary.Delay` 1.5)
      (`self.K2_SetActorLocation` (`self.PlayerCharacter`) (`self.RespawnLocation`) false true)
      (`PlayerCameraManager.StartCameraFade` :`self` (`GameplayStatics.GetPlayerCameraManager` 0) :`FromAlpha` 1.0 :`Duration` 1.5 :`bHoldWhenFinished` true))))

(fn `UserConstructionScript`)