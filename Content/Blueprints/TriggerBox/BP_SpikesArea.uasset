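; Spike trap trigger area that sends the player back to a respawn location when they step into it.
; While enabled, an overlap by the cached player character disables input and raises every BP_Spike in the level, not just nearby ones.
; After a timed camera fade-out, it teleports the player, lowers the spikes, starts the fade-in and restores input.
; DisableZone switches the trap off.
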(event `self.ReceiveBeginPlay`
  (bind _asbp_player_character (cast `/Game/Blueprints/BP_PlayerCharacter` (`GameplayStatics.GetPlayerPawn` 0)))
  (set `self.PlayerCharacter` _asbp_player_character))

(event `self.ReceiveActorBeginOverlap`
  (params (OtherActor :type "Actor Object Reference"))
  (bind _returnvalue (`GameplayStatics.GetPlayerController` 0))
  ;[1 1 1] Handles player respawn
  (if (== OtherActor (`self.PlayerCharacter`))
    (if (`self.SpikesEnabled`)
      (`self.DisableInput` _returnvalue _returnvalue)
      (bind _outactors (`GameplayStatics.GetAllActorsOfClass` "/Game/Blueprints/BlueprintMeshes/BP_Spike.BP_Spike_C"))
      (`/Game/Blueprints/BlueprintMeshes/BP_Spike.SpikeUp` _outactors)
      (`PlayerCameraManager.StartCameraFade` :`self` (`GameplayStatics.GetPlayerCameraManager` 0) :`ToAlpha` 1.0 :`Duration` 2.0 :`bHoldWhenFinished` true)
      (`KismetSystemLibrary.Delay` 2.0)
      (`self.K2_SetActorLocation` (`self.PlayerCharacter`) (`self.RespawnLocation`) false false)
      (`/Game/Blueprints/BlueprintMeshes/BP_Spike.SpikeDown` _outactors)
      (`PlayerCameraManager.StartCameraFade` :`self` (`GameplayStatics.GetPlayerCameraManager` 0) :`FromAlpha` 1.0 :`Duration` 2.0 :`bHoldWhenFinished` true)
      (`self.EnableInput` (`self.PlayerCharacter`) (`GameplayStatics.GetPlayerController` 0))
      (`self.EnableInput` (`GameplayStatics.GetPlayerController` 0) (`GameplayStatics.GetPlayerController` 0)))))

(event `DisableZone`
  (set `self.SpikesEnabled` false))

(fn `UserConstructionScript`)